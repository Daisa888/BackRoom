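; Player controller that sets up Enhanced Input contexts, creates the main pawn HUD and passes possessed pawns to the custom camera manager.
; Interface events drive HUD materials: SAN sets a scaled sanity parameter, while HP lowers a target that a looping timer interpolates the life bar toward.
; Escape or Z opens the game option widget.
; A SwitchInput function toggles between locomotion and show-mesh mapping contexts.
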(event Custom|Update%20Dynamic%20HP
  ;[1 1 1] 角色的数值接口 SAN值默认满格为12  HP默认满血为1
  (bind _returnvalue (Appearance|GetDynamicMaterial (Variables|/Game/TA/01_BP_UI/BP_MainPawnUI.BP_MainPawnUI_C|GetLifebar (Variables|Default|GetMainUI)) :!class /Script/UMG.Image))
  (Rendering|Material|SetScalarParameterValue _returnvalue "血量值" (Math|Interpolation|FInterpTo (Variables|Default|GetCurrent%20HP) (Variables|Default|GetTarget%20HP) (Utilities|Time|GetWorldDeltaSeconds) 1e+01) :!class /Script/Engine.MaterialInstanceDynamic)
  (Variables|Default|SetCurrent%20HP (Math|Interpolation|FInterpTo (Variables|Default|GetCurrent%20HP) (Variables|Default|GetTarget%20HP) (Utilities|Time|GetWorldDeltaSeconds) 1e+01))
  (if (== (Math|Interpolation|FInterpTo (Variables|Default|GetCurrent%20HP) (Variables|Default|GetTarget%20HP) (Utilities|Time|GetWorldDeltaSeconds) 1e+01) (Variables|Default|GetTarget%20HP))
    (Variables|Default|SetLooping false)
    (Utilities|Time|ClearandInvalidateTimerbyHandle (Variables|Default|Get定时器句柄))))

(event Custom|IF_AddHP
  (params (HP :type Float%20%28double-precision%29))
  ;[1 1 1] 角色的数值接口 SAN值默认满格为12  HP默认满血为1
  (Variables|Default|SetLooping true)
  (Variables|Default|SetTarget%20HP (- (Variables|Default|GetTarget%20HP) HP))
  (bind _returnvalue (Utilities|Time|SetTimerbyEvent (delegate Custom|Update%20Dynamic%20HP) 0.02 (Variables|Default|GetLooping)))
  (Variables|Default|Set定时器句柄 _returnvalue))

(event Custom|IF_AddSAN
  (params (SAN :type Float%20%28double-precision%29))
  ;[1 1 1] 角色的数值接口 SAN值默认满格为12  HP默认满血为1
  (Variables|Default|SetSAN (- (Variables|Default|GetSAN) (* SAN 0.255)))
  (bind _returnvalue (Appearance|GetDynamicMaterial (Variables|/Game/TA/01_BP_UI/BP_MainPawnUI.BP_MainPawnUI_C|GetImage_85 (Variables|Default|GetMainUI)) :!class /Script/UMG.Image))
  (Rendering|Material|SetScalarParameterValue _returnvalue "清醒值" (Variables|Default|GetSAN) :!class /Script/Engine.MaterialInstanceDynamic))

(event EventBeginPlay
  (CallFunction|OnAddMappingContext)
  (bind _returnvalue (UserInterface|CreateWidget "/Game/TA/01_BP_UI/BP_MainPawnUI.BP_MainPawnUI_C"))
  (bind _output_get (Variables|Default|SetMainUI _returnvalue))
  (UserInterface|Viewport|AddtoViewport _output_get 0))

(event EventTick
  (params (DeltaSeconds :type Float%20%28single-precision%29))
  ;[1 1 1] 角色的数值接口 SAN值默认满格为12  HP默认满血为1
)

(event EventPossess
  (params (PossessedPawn :type Pawn%20Object%20Reference))
  (bind _ascamera_player_controller (Utilities|Casting|CastToCameraPlayerController (Variables|Default|GetPlayerCameraManager)))
  (Default|OnPossess _ascamera_player_controller PossessedPawn))

(event Input|KeyboardEvents|Escape
  (params (Key :type Key%20Structure :default "None"))
  (:Pressed
    (CallFunction|CreateMainUI1)))

(event Input|KeyboardEvents|Z
  (params (Key :type Key%20Structure :default "None"))
  (:Pressed
    (CallFunction|CreateMainUI1)))

(fn ConstructionScript)

(fn OnAddMappingContext
  (bind _returnvalue (PlayerController|LocalPlayerSubsystems|GetEnhancedInputLocalPlayerSubsystem))
  (Utilities|IsValid _returnvalue
    (:Is%20Valid
      (Input|AddMappingContext _returnvalue "/Game/MyCharacters/Input/IM_Locomotion.IM_Locomotion" 1 "(bIgnoreAllPressedKeysUntilRelease=True,bForceImmediately=False,bNotifyUserSettings=False)")
      (Input|AddMappingContext _returnvalue "/Game/LookAtItem/Input/Contest/IMC_ShowMesh.IMC_ShowMesh" 0 "(bIgnoreAllPressedKeysUntilRelease=True,bForceImmediately=False,bNotifyUserSettings=False)")
      (Input|AddMappingContext _returnvalue "/Game/LookAtItem/Input/Contest/IMC_Torbar.IMC_Torbar" 0 "(bIgnoreAllPressedKeysUntilRelease=True,bForceImmediately=False,bNotifyUserSettings=False)"))))

(fn SwitchInput
  (bind _returnvalue (PlayerController|LocalPlayerSubsystems|GetEnhancedInputLocalPlayerSubsystem))
  (if (Variables|Default|GetSwitchBool)
    (Input|AddMappingContext _returnvalue "/Game/MyCharacters/Input/IM_Locomotion.IM_Locomotion" 0 "(bIgnoreAllPressedKeysUntilRelease=True,bForceImmediately=False,bNotifyUserSettings=False)")
    (Variables|Default|SetSwitchBool false)
    (Input|RemoveMappingContext _returnvalue "/Game/LookAtItem/Input/Contest/IMC_ShowMesh.IMC_ShowMesh" "(bIgnoreAllPressedKeysUntilRelease=True,bForceImmediately=False,bNotifyUserSettings=False)")
    (Input|SetInputModeGameOnly self false)
    (else
      (Input|RemoveMappingContext _returnvalue "/Game/MyCharacters/Input/IM_Locomotion.IM_Locomotion" "(bIgnoreAllPressedKeysUntilRelease=True,bForceImmediately=False,bNotifyUserSettings=False)")
      (Variables|Default|SetSwitchBool true)
      (Input|AddMappingContext _returnvalue "/Game/LookAtItem/Input/Contest/IMC_ShowMesh.IMC_ShowMesh" 0 "(bIgnoreAllPressedKeysUntilRelease=True,bForceImmediately=False,bNotifyUserSettings=False)"))))

(fn CreateMainUI1
  (bind _returnvalue (UserInterface|CreateWidget "/Game/GN/UI/UI_game_Option.UI_game_Option_C"))
  (bind _output_get (Variables|Default|SetUI%20Game%20Option _returnvalue))
  (UserInterface|Viewport|AddtoViewport _output_get 0))

(fn DeleteMainUI1
  (Utilities|IsValid (Variables|Default|GetUI%20Game%20Option)
    (:Is%20Valid
      (Widget|RemovefromParent (Variables|Default|GetUI%20Game%20Option))
      (Variables|Default|SetUI%20Game%20Option 0)
      (Input|SetInputModeGameOnly self false))
    (:Is%20Not%20Valid
      (CallFunction|CreateMainUI1))))