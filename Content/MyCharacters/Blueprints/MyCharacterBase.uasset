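; Base player character with gait and stance locomotion in the style of Advanced Locomotion System, plus item pickup and inventory input.
; Tick derives motion values, resolves gait, then sets speed, acceleration, braking and friction from stance settings and curves.
; Rotation follows control yaw while moving; otherwise it clamps aim offset and turns via the RotationAmount anim curve.
; Input delegates items to BPCTorber and BPCItemComponent; getters expose locomotion state and first-person camera data.
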(event EventBeginPlay
  (CallFunction|BeginPlay)
  (Default|GetMyCharacter (Variables|Default|GetBPC_Torber) self))

(event Collision|EventActorBeginOverlap
  (params (OtherActor :type Actor%20Object%20Reference)))

(event EventTick
  (params (DeltaSeconds :type Float%20%28single-precision%29))
  (Utilities|FlowControl|Sequence
    (:then_0
      (CallFunction|SetEssentialValues)
      (MovementSystem|UpdateCharacterMovement)
      (RotationSystem|UpdateCharacterRotation))
    (:then_1
      (Utilities|FlowControl|Sequence
        (:then_0
          (Variables|CachedVariables|SetPrevious%20Velocity (Transformation|GetVelocity)))
        (:then_1
          (Variables|CachedVariables|SetPrevious%20Aim%20Yaw (.yaw (Pawn|GetControlRotation :!class /Script/Engine.Pawn))))))
    (:then_2
      (Default|OutLineEffect (Variables|Default|GetBPC_Item_Component)))))

(event Custom|RemoveSlot
  (params (Item :type Name%20%28by%20ref%29))
  (bind _bpc_torber (Variables|Default|GetBPC_Torber))
  (Utilities|Array|RemoveItem (Variables|/Game/MyCharacters/Blueprints/BPC_Torber.BPC_Torber_C|GetItemIDList _bpc_torber) Item)
  (Variables|/Game/MyCharacters/Blueprints/BPC_Torber.BPC_Torber_C|SetSelected%20Inventory%20Index _bpc_torber -1))

(event Input|EnhancedActionEvents|EnhancedInputActionIA_PickUp
  (params (ActionValue :type Boolean) (ElapsedSeconds :type Float%20%28double-precision%29) (TriggeredSeconds :type Float%20%28double-precision%29) (InputAction :type Input%20Action%20Object%20Reference :default "/Game/LookAtItem/Input/Action/IA_PickUp.IA_PickUp"))
  (:Started
    (Default|OnPickUP (Variables|Default|GetBPC_Torber))))

(event Input|EnhancedActionEvents|EnhancedInputActionIA_RotateMesh
  (params (ActionValue :type Vector%202D%20Structure) (ElapsedSeconds :type Float%20%28double-precision%29) (TriggeredSeconds :type Float%20%28double-precision%29) (InputAction :type Input%20Action%20Object%20Reference :default "/Game/LookAtItem/Input/Action/IA_RotateMesh.IA_RotateMesh"))
  (Default|RotateMesh (Variables|Default|GetBPC_Torber) (.x ActionValue) (.y ActionValue)))

(event Input|EnhancedActionEvents|EnhancedInputActionIA_Selecter06
  (params (ActionValue :type Boolean) (ElapsedSeconds :type Float%20%28double-precision%29) (TriggeredSeconds :type Float%20%28double-precision%29) (InputAction :type Input%20Action%20Object%20Reference :default "/Game/LookAtItem/Input/Action/IA_Selecter06.IA_Selecter06"))
  (:Started
    (Default|SelectInventoryIndex (Variables|Default|GetBPC_Torber) 5)))

(event Input|EnhancedActionEvents|EnhancedInputActionIA_Selecter07
  (params (ActionValue :type Boolean) (ElapsedSeconds :type Float%20%28double-precision%29) (TriggeredSeconds :type Float%20%28double-precision%29) (InputAction :type Input%20Action%20Object%20Reference :default "/Game/LookAtItem/Input/Action/IA_Selecter07.IA_Selecter07"))
  (:Started
    (Default|SelectInventoryIndex (Variables|Default|GetBPC_Torber) 6)))

(event Input|EnhancedActionEvents|EnhancedInputActionIA_Selecter08
  (params (ActionValue :type Boolean) (ElapsedSeconds :type Float%20%28double-precision%29) (TriggeredSeconds :type Float%20%28double-precision%29) (InputAction :type Input%20Action%20Object%20Reference :default "/Game/LookAtItem/Input/Action/IA_Selecter08.IA_Selecter08"))
  (:Started
    (Default|SelectInventoryIndex (Variables|Default|GetBPC_Torber) 7)))

(event Input|EnhancedActionEvents|EnhancedInputActionIA_Selecter09
  (params (ActionValue :type Boolean) (ElapsedSeconds :type Float%20%28double-precision%29) (TriggeredSeconds :type Float%20%28double-precision%29) (InputAction :type Input%20Action%20Object%20Reference :default "/Game/LookAtItem/Input/Action/IA_Selecter09.IA_Selecter09"))
  (:Started
    (Default|SelectInventoryIndex (Variables|Default|GetBPC_Torber) 8)))

(event Input|EnhancedActionEvents|EnhancedInputActionIA_Selecter00
  (params (ActionValue :type Boolean) (ElapsedSeconds :type Float%20%28double-precision%29) (TriggeredSeconds :type Float%20%28double-precision%29) (InputAction :type Input%20Action%20Object%20Reference :default "/Game/LookAtItem/Input/Action/IA_Selecter00.IA_Selecter00"))
  (:Started
    (Default|SelectInventoryIndex (Variables|Default|GetBPC_Torber) 9)))

(event Input|EnhancedActionEvents|EnhancedInputActionIA_Crouch
  (params (ActionValue :type Boolean) (ElapsedSeconds :type Float%20%28double-precision%29) (TriggeredSeconds :type Float%20%28double-precision%29) (InputAction :type Input%20Action%20Object%20Reference :default "/Game/MyCharacters/Input/Action/IA_Crouch.IA_Crouch"))
  (:Started
    (switch Utilities|FlowControl|Switch|SwitchonStance (Variables|StateValues|GetStance)
      (:NewEnumerator0
        (Variables|StateValues|SetStance "NewEnumerator1"))
      (:NewEnumerator1
        (Variables|StateValues|SetStance "NewEnumerator0")))))

(event Input|EnhancedActionEvents|EnhancedInputActionIA_MouseDown
  (params (ActionValue :type Boolean) (ElapsedSeconds :type Float%20%28double-precision%29) (TriggeredSeconds :type Float%20%28double-precision%29) (InputAction :type Input%20Action%20Object%20Reference :default "/Game/LookAtItem/Input/Action/IA_MouseDown.IA_MouseDown"))
  (:Triggered
    (Variables|/Game/MyCharacters/Blueprints/BPC_Torber.BPC_Torber_C|SetIsMouseDown (Variables|Default|GetBPC_Torber) true))
  (:Completed
    (Variables|/Game/MyCharacters/Blueprints/BPC_Torber.BPC_Torber_C|SetIsMouseDown (Variables|Default|GetBPC_Torber) false)))

(event Input|EnhancedActionEvents|EnhancedInputActionIA_OpenShow
  (params (ActionValue :type Boolean) (ElapsedSeconds :type Float%20%28double-precision%29) (TriggeredSeconds :type Float%20%28double-precision%29) (InputAction :type Input%20Action%20Object%20Reference :default "/Game/LookAtItem/Input/Action/IA_OpenShow.IA_OpenShow"))
  (:Started
    (Default|OnShowMesh (Variables|Default|GetBPC_Torber))))

(event Input|EnhancedActionEvents|EnhancedInputActionIA_LookA
  (params (ActionValue :type Vector%202D%20Structure) (ElapsedSeconds :type Float%20%28double-precision%29) (TriggeredSeconds :type Float%20%28double-precision%29) (InputAction :type Input%20Action%20Object%20Reference :default "/Game/FirstPerson/Input/Actions/IA_LookA.IA_LookA"))
  (Pawn|Input|AddControllerYawInput (.x (stale Input|EnhancedActionEvents|EnhancedInputActionIA_Look ActionValue)))
  (Pawn|Input|AddControllerPitchInput (* (.y (stale Input|EnhancedActionEvents|EnhancedInputActionIA_Look ActionValue)) -1.0)))

(event Input|EnhancedActionEvents|EnhancedInputActionIA_Move
  (params (ActionValue :type Vector%202D%20Structure) (ElapsedSeconds :type Float%20%28double-precision%29) (TriggeredSeconds :type Float%20%28double-precision%29) (InputAction :type Input%20Action%20Object%20Reference :default "/Game/MyCharacters/Input/Action/IA_Move.IA_Move"))
  (bind _returnvalue (Pawn|GetControlRotation :!class /Script/Engine.Pawn))
  (Pawn|Input|AddMovementInput (Math|Vector|GetRightVector (Math|Rotator|MakeRotator (.roll _returnvalue) 0.0 (.yaw _returnvalue))) (.x ActionValue) false)
  (Pawn|Input|AddMovementInput (Math|Vector|GetForwardVector (Math|Rotator|MakeRotator 0.0 0.0 (.yaw (Pawn|GetControlRotation :!class /Script/Engine.Pawn)))) (.y ActionValue) false))

(event Input|EnhancedActionEvents|EnhancedInputActionIA_Look
  (params (ActionValue :type Vector%202D%20Structure) (ElapsedSeconds :type Float%20%28double-precision%29) (TriggeredSeconds :type Float%20%28double-precision%29) (InputAction :type Input%20Action%20Object%20Reference :default "/Game/MyCharacters/Input/Action/IA_Look.IA_Look"))
  (Pawn|Input|AddControllerYawInput (.x ActionValue))
  (Pawn|Input|AddControllerPitchInput (* (.y ActionValue) -1.0)))

(event Input|EnhancedActionEvents|EnhancedInputActionIA_Walk
  (params (ActionValue :type Boolean) (ElapsedSeconds :type Float%20%28double-precision%29) (TriggeredSeconds :type Float%20%28double-precision%29) (InputAction :type Input%20Action%20Object%20Reference :default "/Game/MyCharacters/Input/Action/IA_Walk.IA_Walk"))
  (:Started
    (Variables|StateValues|SetDesired%20Gait "NewEnumerator0")))

(event Input|EnhancedActionEvents|EnhancedInputActionIA_Selecter01
  (params (ActionValue :type Boolean) (ElapsedSeconds :type Float%20%28double-precision%29) (TriggeredSeconds :type Float%20%28double-precision%29) (InputAction :type Input%20Action%20Object%20Reference :default "/Game/LookAtItem/Input/Action/IA_Selecter01.IA_Selecter01"))
  (:Started
    (Default|SelectInventoryIndex (Variables|Default|GetBPC_Torber))))

(event Input|EnhancedActionEvents|EnhancedInputActionIA_Stride
  (params (ActionValue :type Boolean) (ElapsedSeconds :type Float%20%28double-precision%29) (TriggeredSeconds :type Float%20%28double-precision%29) (InputAction :type Input%20Action%20Object%20Reference :default "/Game/MyCharacters/Input/Action/IA_Stride.IA_Stride"))
  (:Triggered
    (Variables|StateValues|SetDesired%20Gait "NewEnumerator2"))
  (:Completed
    (Variables|StateValues|SetDesired%20Gait "NewEnumerator1")))

(event Input|EnhancedActionEvents|EnhancedInputActionIA_Selecter02
  (params (ActionValue :type Boolean) (ElapsedSeconds :type Float%20%28double-precision%29) (TriggeredSeconds :type Float%20%28double-precision%29) (InputAction :type Input%20Action%20Object%20Reference :default "/Game/LookAtItem/Input/Action/IA_Selecter02.IA_Selecter02"))
  (:Started
    (Default|SelectInventoryIndex (Variables|Default|GetBPC_Torber) 1)))

(event Input|EnhancedActionEvents|EnhancedInputActionIA_Selecter03
  (params (ActionValue :type Boolean) (ElapsedSeconds :type Float%20%28double-precision%29) (TriggeredSeconds :type Float%20%28double-precision%29) (InputAction :type Input%20Action%20Object%20Reference :default "/Game/LookAtItem/Input/Action/IA_Selecter03.IA_Selecter03"))
  (:Started
    (Default|SelectInventoryIndex (Variables|Default|GetBPC_Torber) 2)))

(event Input|EnhancedActionEvents|EnhancedInputActionIA_Selecter04
  (params (ActionValue :type Boolean) (ElapsedSeconds :type Float%20%28double-precision%29) (TriggeredSeconds :type Float%20%28double-precision%29) (InputAction :type Input%20Action%20Object%20Reference :default "/Game/LookAtItem/Input/Action/IA_Selecter04.IA_Selecter04"))
  (:Started
    (Default|SelectInventoryIndex (Variables|Default|GetBPC_Torber) 3)))

(event Input|EnhancedActionEvents|EnhancedInputActionIA_Selecter05
  (params (ActionValue :type Boolean) (ElapsedSeconds :type Float%20%28double-precision%29) (TriggeredSeconds :type Float%20%28double-precision%29) (InputAction :type Input%20Action%20Object%20Reference :default "/Game/LookAtItem/Input/Action/IA_Selecter05.IA_Selecter05"))
  (:Started
    (Default|SelectInventoryIndex (Variables|Default|GetBPC_Torber) 4)))

(event Input|KeyboardEvents|1
  (params (Key :type Key%20Structure :default "None"))
  (:Pressed
    (Default|Click (Variables|Default|GetBPC_Item_Component))))

(fn ConstructionScript)

(fn BeginPlay
  (bind _returnvalue (Transformation|GetActorRotation))
  (bind _mesh (Variables|Character|GetMesh))
  (bind _returnvalue_2 (Components|SkeletalMesh|GetAnimInstance _mesh))
  (Utilities|FlowControl|Sequence
    (:then_0
      (Utilities|IsValid _returnvalue_2
        (:Is%20Valid
          (Variables|Default|SetAnim%20Instance _returnvalue_2))))
    (:then_1
      (Variables|RotationSystem|SetTargetRotation _returnvalue)
      (Variables|RotationSystem|SetLast%20Movemenet%20Input%20Rotation _returnvalue))))

(fn SetEssentialValues
  (bind _charactermovement (Variables|Character|GetCharacterMovement))
  (Utilities|FlowControl|Sequence
    (:then_0
      (Variables|EssentialInformation|SetAcceleration (/ (- (Transformation|GetVelocity) (Variables|CachedVariables|GetPrevious%20Velocity)) (Utilities|Time|GetWorldDeltaSeconds))))
    (:then_1
      (bind _output_get (Variables|EssentialInformation|SetSpeed (Math|Vector|VectorLengthXY (Transformation|GetVelocity))))
      (Variables|EssentialInformation|SetIs%20Moving (> _output_get 1.0)))
    (:then_2
      (bind _output_get_2 (Variables|EssentialInformation|SetMovement%20Input%20Amount (/ (Math|Vector|VectorLengthXY (Pawn|Components|CharacterMovement|GetCurrentAcceleration _charactermovement)) (Class|CharacterMovementComponent|GetMaxAcceleration _charactermovement))))
      (bind _output_get_3 (Variables|EssentialInformation|SetHas%20Movement%20Input (> _output_get_2 0.0)))
      (if _output_get_3
        (Variables|RotationSystem|SetLast%20Movemenet%20Input%20Rotation (Math|Conversions|RotationFromXVector (Pawn|Components|CharacterMovement|GetCurrentAcceleration (Variables|Character|GetCharacterMovement))))))
    (:then_3
      (Variables|EssentialInformation|SetAim%20Yaw%20Rate (/ (- (.yaw (Pawn|GetControlRotation :!class /Script/Engine.Pawn)) (Variables|CachedVariables|GetPrevious%20Aim%20Yaw)) (Utilities|Time|GetWorldDeltaSeconds))))))

(fn UpdateCharacterMovement
  (Utilities|FlowControl|Sequence
    (:then_0
      (Variables|StateValues|SetAllowedGait (MovementSystem|GetAllowedGait)))
    (:then_1
      (Variables|StateValues|SetActualGait (MovementSystem|GetActualGait (Variables|StateValues|GetAllowedGait)))
      (if (Utilities|Enum|NotEqual(Enum) (Variables|StateValues|GetActualGait) (Variables|StateValues|GetGait))
        (Variables|StateValues|SetGait (Variables|StateValues|GetActualGait))))
    (:then_2
      (MovementSystem|UpdateDynamicMovementSetting (Variables|StateValues|GetAllowedGait)))))

(fn UpdateCharacterRotation
  (bind _anim_instance (Variables|Default|GetAnim%20Instance))
  (bind _returnvalue (Animation|Curves|GetCurveValue _anim_instance "RotationAmount"))
  (if (RotationSystem|CanUpdateMovingRotation)
    (switch Utilities|FlowControl|Switch|SwitchonGait (Variables|StateValues|GetGait)
      (:NewEnumerator0
        _)
      (:NewEnumerator1
        _)
      (:NewEnumerator2
        _))
    (RotationSystem|SmoothCharacterRotaion (Math|Rotator|MakeRotator 0.0 0.0 (.yaw (Pawn|GetControlRotation :!class /Script/Engine.Pawn))) 5e+02 (RotationSystem|CalculateGroundedRotationRate(pure)))
    (else
      (RotationSystem|LimitRotation -1e+02 1e+02 2e+01)
      (if (> (Math|Float|Absolute(Float) _returnvalue) 0.001)
        (Class|Actor|AddActorWorldRotation (Math|Rotator|MakeRotator 0.0 0.0 (* _returnvalue (Utilities|Time|GetWorldDeltaSeconds) 3e+01)))
        (Variables|RotationSystem|SetTargetRotation (Transformation|GetActorRotation))))))

(fn GetAllowedGait
  (switch Utilities|FlowControl|Switch|SwitchonStance (Variables|StateValues|GetStance)
    (:NewEnumerator0
      (switch Utilities|FlowControl|Switch|SwitchonGait (Variables|StateValues|GetDesired%20Gait)
        (:NewEnumerator0
          (return "NewEnumerator0"))
        (:NewEnumerator1
          (return "NewEnumerator1"))
        (:NewEnumerator2
          ;[1 1 1] 注释
          (return "NewEnumerator2"))))
    (:NewEnumerator1
      (switch Utilities|FlowControl|Switch|SwitchonGait (Variables|StateValues|GetDesired%20Gait)
        (:NewEnumerator0
          (return "NewEnumerator0"))
        (:NewEnumerator1
          _)
        (:NewEnumerator2
          _))
      (return "NewEnumerator1"))))

(fn GetActualGait
  (params (Allowed%20Gait :type Gait%20Enum :default "NewEnumerator0"))
  (bind _movementinfo (Variables|数据表格|GetMovementInfo))
  (LocalVariables|SetLocal%20Walk%20Speed (.walkspeed _movementinfo))
  (LocalVariables|SetLocal%20Run%20Speed (.runspeed _movementinfo))
  (LocalVariables|SetLocal%20Sprint%20Speed (.springspeed _movementinfo))
  (if (>= (Variables|EssentialInformation|GetSpeed) (+ (LocalVariables|GetLocal%20Run%20Speed) 1e+01))
    (switch Utilities|FlowControl|Switch|SwitchonGait (Variables|StateValues|GetAllowedGait)
      (:NewEnumerator0
        _)
      (:NewEnumerator1
        _)
      (:NewEnumerator2
        (return "NewEnumerator2")))
    (return "NewEnumerator1")
    (elif (>= (Variables|EssentialInformation|GetSpeed) (+ (LocalVariables|GetLocal%20Walk%20Speed) 1e+01))
      (return "NewEnumerator1")
      (else
        (return "NewEnumerator0")))))

(fn UpdateDynamicMovementSetting
  (params (AllowedGait :type Gait%20Enum :default "NewEnumerator0"))
  (bind _charactermovement (Variables|Character|GetCharacterMovement))
  (switch Utilities|FlowControl|Switch|SwitchonStance (Variables|StateValues|GetStance)
    (:NewEnumerator0
      (Variables|数据表格|SetMovementInfo (.standing (Variables|DataTable|GetMovement))))
    (:NewEnumerator1
      (Variables|数据表格|SetMovementInfo (.crouching (Variables|DataTable|GetMovement)))))
  (Utilities|FlowControl|Sequence
    (:then_0
      (bind _output_get (Variables|/Script/Engine.CharacterMovementComponent|SetMaxWalkSpeed (Variables|Character|GetCharacterMovement) (Utilities|Select :Index (Variables|StateValues|GetAllowedGait) :NewEnumerator0 (.walkspeed (Variables|数据表格|GetMovementInfo)) :NewEnumerator1 (.runspeed (Variables|数据表格|GetMovementInfo)) :NewEnumerator2 (.springspeed (Variables|数据表格|GetMovementInfo)))))
      (Variables|/Script/Engine.CharacterMovementComponent|SetMaxWalkSpeedCrouched (Variables|Character|GetCharacterMovement) _output_get))
    (:then_1
      (Variables|/Script/Engine.CharacterMovementComponent|SetMaxAcceleration _charactermovement (.x (Math|Curves|GetVectorValue (.movementcurve (Variables|数据表格|GetMovementInfo)) (MovementSystem|GetMappedSpeed))))
      (Variables|/Script/Engine.CharacterMovementComponent|SetBrakingDecelerationWalking _charactermovement (.y (Math|Curves|GetVectorValue (.movementcurve (Variables|数据表格|GetMovementInfo)) (MovementSystem|GetMappedSpeed))))
      (Variables|/Script/Engine.CharacterMovementComponent|SetGroundFriction _charactermovement (.z (Math|Curves|GetVectorValue (.movementcurve (Variables|数据表格|GetMovementInfo)) (MovementSystem|GetMappedSpeed)))))))

(fn CanUpdateMovingRotation
  (return (and (or (and (Variables|EssentialInformation|GetIs%20Moving) (Variables|EssentialInformation|GetHas%20Movement%20Input)) (> (Variables|EssentialInformation|GetSpeed) 1.5e+02)) (not (Class|Character|HasAnyRootMotion)))))

(fn SmoothCharacterRotaion
  (params (Target :type Rotator) (Target%20Inter%20Speed%28Const%29 :type Float%20%28double-precision%29) (Actor%20Interp%20Speed%28Smooth%29 :type Float%20%28double-precision%29))
  (Variables|RotationSystem|SetTargetRotation (Class|KismetMathLibrary|RInterptoConstant (Variables|RotationSystem|GetTargetRotation) Target (Utilities|Time|GetWorldDeltaSeconds) Target%20Inter%20Speed%28Const%29))
  (Transformation|SetActorRotation (Math|Interpolation|RInterpTo (Transformation|GetActorRotation) (Variables|RotationSystem|GetTargetRotation) (Utilities|Time|GetWorldDeltaSeconds) Actor%20Interp%20Speed%28Smooth%29)))

(fn CalculateGroundedRotationRate(pure)
  (return (* (Math|Curves|GetFloatValue (.rotationratecurve (Variables|数据表格|GetMovementInfo)) (MovementSystem|GetMappedSpeed)) (Math|Float|MapRangeClamped (Variables|EssentialInformation|GetAim%20Yaw%20Rate) 0.0 3e+02 1.0 3.0))))

(fn LimitRotation
  (params (Aim%20Yaw%20Min :type Float%20%28double-precision%29) (Aim%20Yaw%20Max :type Float%20%28double-precision%29) (Interp%20Speed :type Float%20%28double-precision%29))
  (bind _returnvalue (Pawn|GetControlRotation :!class /Script/Engine.Pawn))
  (bind _returnvalue_2 (Transformation|GetActorRotation))
  (bind _returnvalue_3 (Pawn|GetControlRotation :!class /Script/Engine.Pawn))
  (bind _returnvalue_4 (Math|Rotator|Delta(Rotator) _returnvalue _returnvalue_2))
  (if (not (Math|Float|InRange(Float) (.yaw _returnvalue_4) Aim%20Yaw%20Min Aim%20Yaw%20Max))
    (RotationSystem|SmoothCharacterRotaion (Math|Rotator|MakeRotator 0.0 0.0 (Math|Float|SelectFloat (+ (.yaw _returnvalue_3) Aim%20Yaw%20Min) (+ (.yaw _returnvalue_3) Aim%20Yaw%20Max) (> (.yaw _returnvalue_4) 0.0))) 0.0 Interp%20Speed)))

(fn GetMappedSpeed
  (bind _movementinfo (Variables|数据表格|GetMovementInfo))
  (bind _speed (Variables|EssentialInformation|GetSpeed))
  (LocalVariables|SetLocWalkSpeed (.walkspeed _movementinfo))
  (LocalVariables|SetLocRunSpeed (.runspeed _movementinfo))
  (LocalVariables|SetLocSprintSpeed (.springspeed _movementinfo))
  (return (select (> (Variables|EssentialInformation|GetSpeed) (LocalVariables|GetLocRunSpeed)) (Math|Float|MapRangeClamped _speed (LocalVariables|GetLocRunSpeed) (LocalVariables|GetLocSprintSpeed) 2.0 3.0) (select (> (Variables|EssentialInformation|GetSpeed) (LocalVariables|GetLocWalkSpeed)) (Math|Float|MapRangeClamped _speed (LocalVariables|GetLocWalkSpeed) (LocalVariables|GetLocRunSpeed) 1.0 2.0) (Math|Float|MapRangeClamped _speed 0.0 (LocalVariables|GetLocWalkSpeed) 0.0 1.0)))))

(fn BPIGetCurrentStates
  (return (Variables|StateValues|GetStance) (Variables|StateValues|GetActualGait) false))

(fn BPIGetEssentialValues
  (return (Transformation|GetVelocity) (Variables|EssentialInformation|GetAcceleration) (Pawn|Components|CharacterMovement|GetCurrentAcceleration (Variables|Character|GetCharacterMovement)) (Variables|EssentialInformation|GetIs%20Moving) (Variables|EssentialInformation|GetHas%20Movement%20Input) (Variables|EssentialInformation|GetSpeed) (Variables|EssentialInformation|GetMovement%20Input%20Amount) (Pawn|GetControlRotation :!class /Script/Engine.Pawn) (Variables|EssentialInformation|GetAim%20Yaw%20Rate)))

(fn GetCameraParameters
  (return (Variables|CameraSystem|GetFirst%20Person%20FOV)))

(fn GetFPCameraTarget
  (return (Transformation|GetSocketLocation (Variables|Character|GetMesh) "FP_Camera")))