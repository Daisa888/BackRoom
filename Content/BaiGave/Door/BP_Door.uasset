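; BP_Door is a lockable physics-driven door actor.
; On BeginPlay it reads the Locked flag and turns physics simulation on the Door component off when locked and on when unlocked.
; SetDoorLocked and SetDoorUnLocked update the flag and toggle the same simulation, so an unlocked door moves by physics and a locked one stops simulating.
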(event EventBeginPlay
  (bind _door (Variables|Default|GetDoor))
  (if (Variables|Default|GetLocked?)
    (Physics|SetSimulatePhysics _door false)
    (else
      (Physics|SetSimulatePhysics _door true))))

(event Collision|EventActorBeginOverlap
  (params (OtherActor :type Actor%20Object%20Reference)))

(event EventTick
  (params (DeltaSeconds :type Float%20%28single-precision%29)))

(fn ConstructionScript)

(fn SetDoorLocked
  (Variables|Default|SetLocked? true)
  (Physics|SetSimulatePhysics (Variables|Default|GetDoor) false))

(fn SetDoorUnLocked
  (Variables|Default|SetLocked? false)
  (Physics|SetSimulatePhysics (Variables|Default|GetDoor) true))