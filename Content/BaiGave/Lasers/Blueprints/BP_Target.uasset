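; BP_Target is a laser target actor that shows its activation state through color.
; On BeginPlay it creates a dynamic instance of MI_Laser, applies it to the static mesh and sets the Color parameter to DefaultColor.
; Activate and deactivate events from its AC_Handler component switch that parameter between TargetColor and DefaultColor.
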(event ActivateHandler(AC_Handler)
  (params (Instigater :type AC%20Handler%20Object%20Reference))
  (Rendering|Material|SetVectorParameterValue (Variables|Default|GetMI_Laser) "Color" (Variables|Default|GetTargetColor) :!class /Script/Engine.MaterialInstanceDynamic))

(event DeactivateHandler(AC_Handler)
  (params (Instigater :type AC%20Handler%20Object%20Reference))
  (Rendering|Material|SetVectorParameterValue (Variables|Default|GetMI_Laser) "Color" (Variables|Default|GetDefaultColor) :!class /Script/Engine.MaterialInstanceDynamic))

(event EventBeginPlay
  (bind _returnvalue (Rendering|Material|CreateDynamicMaterialInstance "/Game/BaiGave/Lasers/Materials/MI_Laser.MI_Laser" "None" "None" :!class /Script/Engine.KismetMaterialLibrary))
  (Variables|Default|SetMI_Laser _returnvalue)
  (Rendering|Material|SetMaterial (Variables|Default|GetStaticMesh) 0 (Variables|Default|GetMI_Laser))
  (Rendering|Material|SetVectorParameterValue (Variables|Default|GetMI_Laser) "Color" (Variables|Default|GetDefaultColor) :!class /Script/Engine.MaterialInstanceDynamic))

(event Collision|EventActorBeginOverlap
  (params (OtherActor :type Actor%20Object%20Reference)))

(event EventTick
  (params (DeltaSeconds :type Float%20%28single-precision%29)))

(fn ConstructionScript)