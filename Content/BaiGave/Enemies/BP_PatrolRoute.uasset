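; BP_PatrolRoute is an enemy patrol route actor that serves world-space waypoints from a PatrolRoute spline.
; IncrementPatrolRoute steps PatrolIndex by Direction and, on hitting the last point's index, immediately sets it to -1 and raises the End flag.
; GetSplinePointWorldLocation returns the point at the current index, and ResetSplinePoint restores the index to -1 and clears End.
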(event Custom|IncrementPatrolRoute
  (bind _output_get (Variables|Default|SetPatrolIndex (+ (Variables|Default|GetPatrolIndex) (Variables|Default|GetDirection))))
  (if (== _output_get (- (Spline|GetNumberOfSplinePoints (Variables|Default|GetPatrolRoute)) 1))
    (Variables|Default|SetPatrolIndex -1)
    (Variables|Default|SetEnd? true)))

(event EventBeginPlay)

(event Collision|EventActorBeginOverlap
  (params (OtherActor :type Actor%20Object%20Reference)))

(event EventTick
  (params (DeltaSeconds :type Float%20%28single-precision%29)))

(fn ConstructionScript)

(fn GetSplinePointWorldLocation
  (return (Spline|GetLocationatSplinePoint (Variables|Default|GetPatrolRoute) (Variables|Default|GetPatrolIndex) "World")))

(fn ResetSplinePoint
  (Variables|Default|SetPatrolIndex -1)
  (Variables|Default|SetEnd? false))