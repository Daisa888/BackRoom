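; BP_NoiseTrigger is a box trigger that has the player character make noise at the box's location when something overlaps it.
; Begin overlap skips actors whose class is exactly BP_Enemy_Base, then calls NoiseMaker on player 0's MyCharacterBase, whoever the overlapper is.
; A Hitted flag blocks repeat noise until a short delay after an end overlap re-arms it.
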(event OnComponentBeginOverlap(Box)
  (params (OverlappedComponent :type Primitive%20Component%20Object%20Reference) (OtherActor :type Actor%20Object%20Reference) (OtherComp :type Primitive%20Component%20Object%20Reference) (OtherBodyIndex :type Integer) (bFromSweep :type Boolean) (SweepResult :type Hit%20Result%20Structure%20%28by%20ref%29))
  (if (not (== (Utilities|GetClass OtherActor) "/Game/BaiGave/Enemies/BP_Enemy_Base.BP_Enemy_Base_C"))
    (if (not (Variables|Default|GetHitted?))
      (bind _asmy_character_base (Utilities|Casting|CastToMyCharacterBase (Game|GetPlayerCharacter 0)))
      (Default|NoiseMaker _asmy_character_base (Transformation|GetWorldLocation (Variables|Default|GetBox)))
      (Variables|Default|SetHitted? true)
      (Development|PrintString "hit"))))

(event OnComponentEndOverlap(Box)
  (params (OverlappedComponent :type Primitive%20Component%20Object%20Reference) (OtherActor :type Actor%20Object%20Reference) (OtherComp :type Primitive%20Component%20Object%20Reference) (OtherBodyIndex :type Integer))
  (if (not (== (Utilities|GetClass 0) "/Game/BaiGave/Enemies/BP_Enemy_Base.BP_Enemy_Base_C"))
    (if (Variables|Default|GetHitted?)
      (Utilities|FlowControl|Delay 5.0)
      (Variables|Default|SetHitted? false))))

(event EventBeginPlay)

(event Collision|EventActorBeginOverlap
  (params (OtherActor :type Actor%20Object%20Reference)))

(event EventTick
  (params (DeltaSeconds :type Float%20%28single-precision%29)))

(fn ConstructionScript)