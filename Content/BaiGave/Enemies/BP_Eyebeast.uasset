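; BP_Eyebeast is an enemy whose static mesh patrols back and forth along its forward axis.
; On BeginPlay, a debug-drawn line trace sets the far endpoint at Distance, or slightly short of a blocking hit.
; After a short delay, a looping timer drives a timeline that interpolates between endpoints, scaling play rate by Speed over path length.
; A FlipFlop on timeline completion toggles Arrived, switching between play and reverse.
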(event Custom|Move
  (Components|Timeline|SetPlayRate (Variables|Default|Get时间轴) (/ (Variables|Default|GetSpeed) (Math|Vector|VectorLength (- (Variables|Default|GetLoc2) (Variables|Default|GetLoc1)))))
  (if (Variables|Default|GetArrived?)
    (bind _新建轨道_0 (Timeline|时间轴 Reverse)
      (:Update
        (Transformation|SetWorldLocation (Variables|Default|GetStaticMesh) (+ (* (- (Variables|Default|GetLoc2) (Variables|Default|GetLoc1)) _新建轨道_0) (Variables|Default|GetLoc1)) false false))
      (:Finished
        (Utilities|FlowControl|FlipFlop
          (:A
            (Variables|Default|SetArrived? true))
          (:B
            (Variables|Default|SetArrived? false)))))
    (else
      (Timeline|时间轴 Play))))

(event Custom|WallMove
  (Utilities|FlowControl|Delay 1.0)
  (Utilities|Time|SetTimerbyEvent (delegate Custom|Move) 0.025 true))

(event EventBeginPlay
  (bind _staticmesh (Variables|Default|GetStaticMesh))
  (bind _staticmesh_2 (Variables|Default|GetStaticMesh))
  (bind _distance (Variables|Default|GetDistance))
  (bind _returnvalue (Transformation|GetWorldLocation _staticmesh_2))
  (bind _returnvalue_2 (Transformation|GetWorldLocation _staticmesh))
  (bind _returnvalue_3 (Math|Vector|GetForwardVector _staticmesh))
  (bind _returnvalue_4 (* _returnvalue_3 _distance))
  (bind _returnvalue_5 (+ _returnvalue_4 _returnvalue_2))
  (Variables|Default|SetLoc1 (Math|Vector|MakeVector (.x _returnvalue) (.y _returnvalue) (.z _returnvalue)))
  (bind _outhit (Collision|LineTraceByChannel _returnvalue_2 _returnvalue_5 "TraceTypeQuery1" false 0 "Persistent"))
  (if (.bBlockingHit (Collision|BreakHitResult _outhit))
    (Variables|Default|SetLoc2 (- (.Location (Collision|BreakHitResult _outhit)) (* _returnvalue_3 50)))
    (CallFunction|WallMove)
    (else
      (Variables|Default|SetLoc2 _returnvalue_5)
      (CallFunction|WallMove))))

(fn ConstructionScript)