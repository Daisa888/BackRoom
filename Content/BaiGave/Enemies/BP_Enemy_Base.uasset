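; Base enemy character Blueprint that supplies shared accessors and actions, apparently for AI logic to call.
; Attack plays a rifle shoot montage on the mesh and fires the OnAttackEnd dispatcher when it completes or is interrupted.
; Getters expose its Door and PatrolRoute references.
; SetMovementSpeed maps a gait enum from idle to sprinting onto the character's max walk speed and returns it.
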(event Custom|Attack
  (Animation|Montage|PlayMontage (Variables|Character|GetMesh) "/Game/FirstPersonArms/Animations/FP_Rifle_Shoot_Montage.FP_Rifle_Shoot_Montage"
    (:OnCompleted
      _)
    (:OnInterrupted
      _))
  (Default|CallOnAttackEnd))

(fn ConstructionScript)

(fn GetDoor
  (return (Variables|Default|GetDoor)))

(fn GetPatrolRoute
  (return (Variables|Default|GetPatrolRoute)))

(fn SetMovementSpeed
  (params (Speed :type E_MovementSpeed%20Enum :default "NewEnumerator0"))
  (bind _output_get (Variables|/Script/Engine.CharacterMovementComponent|SetMaxWalkSpeed (Variables|Character|GetCharacterMovement) (Utilities|Select :Index Speed :NewEnumerator0 0.0 :NewEnumerator1 1e+02 :NewEnumerator2 3e+02 :NewEnumerator3 5e+02)))
  (return _output_get))