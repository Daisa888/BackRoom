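; Clickable button actor that makes its target cabinet pull out the first three entries of its cube array in sequence.
; On click, it calls PullOut on each cube in turn, with a fixed delay after each call.
; Its own Pressed flag and the cabinet's CanPull flag block new pulls until the sequence finishes, then both reset.
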(event EventBeginPlay)

(event Collision|EventActorBeginOverlap
  (params (OtherActor :type Actor%20Object%20Reference)))

(event EventTick
  (params (DeltaSeconds :type Float%20%28single-precision%29)))

(event EventClicked
  (params (C :type Scene%20Component%20Object%20Reference) (O :type Actor%20Object%20Reference))
  (bind _targetcabinet (Variables|Default|GetTargetCabinet))
  (bind _cubearray (Variables|/Game/BaiGave/Cabinet/BP_Cabinet.BP_Cabinet_C|GetCubeArray _targetcabinet))
  (if (not (Variables|Default|GetPressed?))
    (if (Variables|/Game/BaiGave/Cabinet/BP_Cabinet.BP_Cabinet_C|GetCanPull? _targetcabinet)
      (Variables|Default|SetPressed? true)
      (Variables|/Game/BaiGave/Cabinet/BP_Cabinet.BP_Cabinet_C|SetCanPull? _targetcabinet false)
      (Default|PullOut _targetcabinet (Utilities|Array|Get(acopy) _cubearray))
      (Utilities|FlowControl|Delay 2.0)
      (Default|PullOut _targetcabinet (Utilities|Array|Get(acopy) _cubearray 1))
      (Utilities|FlowControl|Delay 2.0)
      (Default|PullOut _targetcabinet (Utilities|Array|Get(acopy) _cubearray 2))
      (Utilities|FlowControl|Delay 2.0)
      (Variables|Default|SetPressed? false)
      (Variables|/Game/BaiGave/Cabinet/BP_Cabinet.BP_Cabinet_C|SetCanPull? (Variables|Default|GetTargetCabinet) true))))

(fn ConstructionScript)