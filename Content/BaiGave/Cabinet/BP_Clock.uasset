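; Interactive clock actor that the player can click to focus on and set by turning its hands with scroll events.
; Each click alternates between blending the view to the clock with movement and look locked, and back to the passed object, updating its item component's focus.
; Scrolling steps the hour angle and derives the minute hand from its remainder within each hour.
; Mouse-hover highlighting and cursor toggling are present but unconnected.
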(event EventBeginPlay
  (|CallParentFunction) ; 此节点被禁用，将不会被调用。\n从引脚连出引线来编译功能。
)

(event Collision|EventActorBeginOverlap
  (params (OtherActor :type Actor%20Object%20Reference))
  (|CallParentFunction OtherActor) ; 此节点被禁用，将不会被调用。\n从引脚连出引线来编译功能。
)

(event EventTick
  (params (DeltaSeconds :type Float%20%28single-precision%29))
  (|CallParentFunction DeltaSeconds))

(event EventClicked
  (params (C :type Scene%20Component%20Object%20Reference) (O :type Actor%20Object%20Reference))
  (bind _returnvalue (Game|GetPlayerController 0))
  ;[1 1 1] 被点击后事件
  (if (not (Variables|Default|GetIsMoveingCamera?))
    (Variables|Default|SetItemComponent (Actor|GetComponentbyClass O "/Game/FirstPerson/Blueprints/BPC_Item_Component.BPC_Item_Component_C"))
    (Variables|Default|SetIsMoveingCamera? true)
    (Variables|Default|SetO O)
    (Utilities|FlowControl|FlipFlop
      (:A
        (Variables|/Game/MyCharacters/Camera/CameraPlayerController.CameraPlayerController_C|SetIs%20View? (.AsCamera%20Player%20Controller (Utilities|Casting|CastToCameraPlayerController (Game|GetPlayerCameraManager 0))) false)
        (Variables|/Game/FirstPerson/Blueprints/BPC_Item_Component.BPC_Item_Component_C|SetIsFocusing? (Variables|Default|GetItemComponent) true)
        (Variables|/Game/FirstPerson/Blueprints/BPC_Item_Component.BPC_Item_Component_C|SetFocusTarget (Variables|Default|GetItemComponent) self)
        (Game|Player|SetViewTargetwithBlend _returnvalue self 1.0 "VTBlend_Linear" 0.0 false)
        (Input|SetIgnoreMoveInput _returnvalue true)
        (Input|SetIgnoreLookInput _returnvalue true)
        (Utilities|FlowControl|Delay 1.0)
        (Variables|Default|SetIsMoveingCamera? false))
      (:B
        (Game|Player|SetViewTargetwithBlend _returnvalue (Variables|Default|GetO) 1.0 "VTBlend_Linear" 0.0 false)
        (Utilities|FlowControl|Delay 1.0)
        (Input|SetIgnoreMoveInput _returnvalue false)
        (Input|SetIgnoreLookInput _returnvalue false)
        (Variables|Default|SetIsMoveingCamera? false)
        (Variables|/Game/FirstPerson/Blueprints/BPC_Item_Component.BPC_Item_Component_C|SetIsFocusing? (Variables|Default|GetItemComponent) false)
        (Variables|/Game/FirstPerson/Blueprints/BPC_Item_Component.BPC_Item_Component_C|SetFocusTarget (Variables|Default|GetItemComponent) 0)
        (Variables|/Game/MyCharacters/Camera/CameraPlayerController.CameraPlayerController_C|SetIs%20View? (.AsCamera%20Player%20Controller (Utilities|Casting|CastToCameraPlayerController (Game|GetPlayerCameraManager 0))) false)))))

(event EventScrollDown
  (bind _output_get (Variables|Default|SetHAngle (+ (Variables|Default|GetHAngle) -2.0)))
  (Transformation|SetWorldRotation (Variables|Default|GetHourHand) (Math|Rotator|MakeRotator 0.0 _output_get 0.0) false false)
  (Transformation|SetWorldRotation (Variables|Default|GetMinuteHand) (Math|Rotator|MakeRotator 0.0 (CallFunction|ConvertHourAngletoMinuteAngle (Variables|Default|GetHAngle)) 0.0) false false))

(event EventScrollUp
  (bind _output_get (Variables|Default|SetHAngle (+ (Variables|Default|GetHAngle) 2.0)))
  (Transformation|SetWorldRotation (Variables|Default|GetHourHand) (Math|Rotator|MakeRotator 0.0 _output_get 0.0) false false)
  (Transformation|SetWorldRotation (Variables|Default|GetMinuteHand) (Math|Rotator|MakeRotator 0.0 (CallFunction|ConvertHourAngletoMinuteAngle (Variables|Default|GetHAngle)) 0.0) false false))

(fn ConstructionScript
  (|CallParentFunction))

(fn ConvertMinuteAngletoHourAngle
  (params (MAngle :type Float%20%28double-precision%29))
  (return (/ (/ MAngle 12.0) 3.6e+02)))

(fn ConvertHourAngletoMinuteAngle
  (params (HAngle :type Float%20%28double-precision%29))
  (return (* (.Remainder (Math|Float|Division(WholeandRemainder) HAngle 3e+01)) 12.0)))