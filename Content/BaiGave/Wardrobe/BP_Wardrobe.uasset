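; Wardrobe actor with two clickable doors that serves as a player hiding spot.
; Clicks toggle each door, with short timers starting per-motion timelines that swing its yaw; every speed adjustment targets only Door2's opening timeline.
; A box overlap tracks the player inside, clearing only after a polled distance check exceeds a threshold on exit.
; Hiding sets IsHiding on the player's BPC_Item_Component only while inside with both doors closed.
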(event OnComponentBeginOverlap(Box)
  (params (OverlappedComponent :type Primitive%20Component%20Object%20Reference) (OtherActor :type Actor%20Object%20Reference) (OtherComp :type Primitive%20Component%20Object%20Reference) (OtherBodyIndex :type Integer) (bFromSweep :type Boolean) (SweepResult :type Hit%20Result%20Structure%20%28by%20ref%29))
  (Utilities|Casting|CastToMyCharacterBase OtherActor)
  (if (not (Variables|Default|GetPlayerInWardrobe?))
    (Variables|Default|SetPlayerInWardrobe? true)
    (CallFunction|Hiding?)))

(event OnComponentEndOverlap(Box)
  (params (OverlappedComponent :type Primitive%20Component%20Object%20Reference) (OtherActor :type Actor%20Object%20Reference) (OtherComp :type Primitive%20Component%20Object%20Reference) (OtherBodyIndex :type Integer))
  (Variables|Default|SetPlayer OtherActor)
  (if (Variables|Default|GetPlayerInWardrobe?) :!label _label
    (if (<= (Math|Vector|Distance(Vector) (Transformation|GetActorLocation (Variables|Default|GetPlayer)) (Transformation|GetWorldLocation (Variables|Default|GetBox))) 3.5e+02)
      (Utilities|FlowControl|Delay 0.1)
      (goto _label)
      (else
        (Variables|Default|SetPlayerInWardrobe? false)
        (CallFunction|Hiding?)))))

(event Custom|CustomEvent_1
  (Components|Timeline|SetPlayRate (Variables|Default|Get时间轴) (/ (Variables|Default|GetSpeed) (Math|Float|Absolute(Float) (- (Variables|Default|GetRot0) (Variables|Default|GetRot1)))))
  (bind _新建轨道_0 (Timeline|时间轴_0 ReverseFromEnd)
    (:Update
      (Transformation|SetRelativeRotation (stale Custom|D1Close 目标) (Math|Rotator|MakeRotator 0.0 0.0 (+ (* _新建轨道_0 (Variables|Default|GetRot1)) (Variables|Default|GetRot0))) false false))))

(event Custom|D2Open
  (params (目标 :type Scene%20Component%20Object%20Reference) (Rot1 :type Float%20%28double-precision%29))
  (if (Utilities|Operators|EqualEqual :A (Variables|/Script/Engine.SceneComponent|GetRelativeRotation 目标))
    (Variables|Default|SetRot0_0 0.0)
    (Variables|Default|SetRot1_0 Rot1)
    (Utilities|Time|SetTimerbyEvent (delegate Custom|Move) 0.025)))

(event Custom|Move
  (Components|Timeline|SetPlayRate (Variables|Default|Get时间轴) (/ (Variables|Default|GetSpeed) (Math|Float|Absolute(Float) (- (Variables|Default|GetRot0_0) (Variables|Default|GetRot1_0)))))
  (bind _新建轨道_0 (Timeline|时间轴 PlayFromStart)
    (:Update
      (Transformation|SetRelativeRotation (stale Custom|D2Open 目标) (Math|Rotator|MakeRotator 0.0 0.0 (+ (* _新建轨道_0 (Variables|Default|GetRot1_0)) (Variables|Default|GetRot0_0))) false false))))

(event Custom|CustomEvent_2
  (Components|Timeline|SetPlayRate (Variables|Default|Get时间轴) (/ (Variables|Default|GetSpeed) (Math|Float|Absolute(Float) (- (Variables|Default|GetRot0_0) (Variables|Default|GetRot1_0)))))
  (bind _新建轨道_0 (Timeline|时间轴_1 ReverseFromEnd)
    (:Update
      (Transformation|SetRelativeRotation (stale Custom|D2Close 目标) (Math|Rotator|MakeRotator 0.0 0.0 (+ (* _新建轨道_0 (Variables|Default|GetRot1_0)) (Variables|Default|GetRot0_0))) false false))))

(event Custom|D2Close
  (params (目标 :type Scene%20Component%20Object%20Reference) (B :type Rotator))
  (if (Utilities|Operators|EqualEqual (Variables|/Script/Engine.SceneComponent|GetRelativeRotation 目标) B 5.0)
    (Variables|Default|SetRot0_0 0.0)
    (Variables|Default|SetRot1_0 (.Yaw (Math|Rotator|BreakRotator B)))
    (Utilities|Time|SetTimerbyEvent (delegate Custom|CustomEvent_2) 0.025)))

(event Custom|D1Open
  (params (目标 :type Scene%20Component%20Object%20Reference) (Rot1 :type Float%20%28double-precision%29))
  (if (Utilities|Operators|EqualEqual :A (Variables|/Script/Engine.SceneComponent|GetRelativeRotation 目标))
    (Variables|Default|SetRot0 0.0)
    (Variables|Default|SetRot1 Rot1)
    (Utilities|Time|SetTimerbyEvent (delegate Custom|CustomEvent_3) 0.025)))

(event Custom|CustomEvent_3
  (Components|Timeline|SetPlayRate (Variables|Default|Get时间轴) (/ (Variables|Default|GetSpeed) (Math|Float|Absolute(Float) (- (Variables|Default|GetRot0) (Variables|Default|GetRot1)))))
  (bind _新建轨道_0 (Timeline|时间轴_2 PlayFromStart)
    (:Update
      (Transformation|SetRelativeRotation (stale Custom|D1Open 目标) (Math|Rotator|MakeRotator 0.0 0.0 (+ (* _新建轨道_0 (Variables|Default|GetRot1)) (Variables|Default|GetRot0))) false false))))

(event Custom|D1Close
  (params (目标 :type Scene%20Component%20Object%20Reference) (B :type Rotator))
  (if (Utilities|Operators|EqualEqual (Variables|/Script/Engine.SceneComponent|GetRelativeRotation 目标) B 5.0)
    (Variables|Default|SetRot0 0.0)
    (Variables|Default|SetRot1 (.Yaw (Math|Rotator|BreakRotator B)))
    (Utilities|Time|SetTimerbyEvent (delegate Custom|CustomEvent_1) 0.025)))

(event EventBeginPlay
  (|CallParentFunction) ; 此节点被禁用，将不会被调用。\n从引脚连出引线来编译功能。
)

(event Collision|EventActorBeginOverlap
  (params (OtherActor :type Actor%20Object%20Reference))
  (|CallParentFunction OtherActor) ; 此节点被禁用，将不会被调用。\n从引脚连出引线来编译功能。
)

(event EventClicked
  (params (C :type Scene%20Component%20Object%20Reference) (O :type Actor%20Object%20Reference))
  (bind _door1 (Variables|组件|GetDoor1))
  (bind _door2 (Variables|组件|GetDoor2))
  (if (== C (Variables|组件|GetDoor1))
    (if (Variables|Default|GetD1Open?)
      (CallFunction|CloseDoor _door1)
      (else
        (CallFunction|OpenDoor _door1)))
    (elif (== C (Variables|组件|GetDoor2))
      (if (Variables|默认|GetD2Open?)
        (CallFunction|CloseDoor _door2)
        (else
          (CallFunction|OpenDoor _door2))))))

(fn ConstructionScript
  (|CallParentFunction))

(fn OpenDoor
  (params (InputPin :type Static%20Mesh%20Component%20Object%20Reference))
  (if (== InputPin (Variables|组件|GetDoor1))
    (Variables|Default|SetD1Open? true)
    (CallFunction|D1Open InputPin 9e+01)
    (CallFunction|Hiding?)
    (elif (== InputPin (Variables|组件|GetDoor2))
      (Variables|默认|SetD2Open? true)
      (CallFunction|D2Open InputPin -9e+01)
      (CallFunction|Hiding?))))

(fn CloseDoor
  (params (InputPin :type Static%20Mesh%20Component%20Object%20Reference))
  (if (== InputPin (Variables|组件|GetDoor1))
    (Variables|Default|SetD1Open? false)
    (CallFunction|D1Close InputPin "0.000000,90.000000,0.000000")
    (CallFunction|Hiding?)
    (elif (== InputPin (Variables|组件|GetDoor2))
      (Variables|默认|SetD2Open? false)
      (CallFunction|D2Close InputPin "0.000000,-90.000000,0.000000")
      (CallFunction|Hiding?))))

(fn Hiding?
  (bind _returnvalue (Game|GetPlayerCharacter 0))
  (bind _returnvalue_2 (Actor|GetComponentbyClass _returnvalue "/Game/FirstPerson/Blueprints/BPC_Item_Component.BPC_Item_Component_C"))
  (if (Variables|Default|GetPlayerInWardrobe?)
    (if (and (not (Variables|Default|GetD1Open?)) (not (Variables|默认|GetD2Open?)))
      (Variables|/Game/FirstPerson/Blueprints/BPC_Item_Component.BPC_Item_Component_C|SetIsHiding? _returnvalue_2 true)
      (Development|PrintText "Hello")
      (else
        (Variables|/Game/FirstPerson/Blueprints/BPC_Item_Component.BPC_Item_Component_C|SetIsHiding? _returnvalue_2 false)))
    (else
      (Variables|/Game/FirstPerson/Blueprints/BPC_Item_Component.BPC_Item_Component_C|SetIsHiding? _returnvalue_2 false))))