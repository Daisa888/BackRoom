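; BP_Door10 is a one-shot swinging door for the dynamic level spawning system, placed under a parent actor.
; Its Open event plays a timeline once that yaws the Scene component up to 90 degrees, scaled by the track value.
; The first player overlap with Box reverses a second timeline to swing it back, then sends IFDynamicSpawnLevelMessage to the parent actor when finished.
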(event OnComponentBeginOverlap(Box)
  (params (OverlappedComponent :type Primitive%20Component%20Object%20Reference) (OtherActor :type Actor%20Object%20Reference) (OtherComp :type Primitive%20Component%20Object%20Reference) (OtherBodyIndex :type Integer) (bFromSweep :type Boolean) (SweepResult :type Hit%20Result%20Structure%20%28by%20ref%29))
  (if (== OtherActor (Game|GetPlayerCharacter 0))
    (Utilities|FlowControl|DoOnce false
      (:Completed
        (bind _新建轨道_0 (Timeline|时间轴_0 ReverseFromEnd)
          (:Update
            (Transformation|SetRelativeRotation (Variables|Default|GetScene) (Math|Rotator|MakeRotator 0.0 0.0 (* _新建轨道_0 9e+01)) false false))
          (:Finished
            (Class|IFDoor|IFDynamicSpawnLevel(Message) (Actor|GetParentActor))))))))

(event EventBeginPlay)

(event Collision|EventActorBeginOverlap
  (params (OtherActor :type Actor%20Object%20Reference)))

(event EventTick
  (params (DeltaSeconds :type Float%20%28single-precision%29)))

(event EventOpen
  (params (SMC :type Static%20Mesh%20Component%20Object%20Reference))
  (Utilities|FlowControl|DoOnce false
    (:Completed
      (bind _新建轨道_0 (Timeline|时间轴 PlayFromStart)
        (:Update
          (Transformation|SetRelativeRotation (Variables|Default|GetScene) (Math|Rotator|MakeRotator 0.0 0.0 (* _新建轨道_0 9e+01)) false false))))))

(event Input|KeyboardEvents|H
  (params (Key :type Key%20Structure :default "None")))

(fn ConstructionScript)