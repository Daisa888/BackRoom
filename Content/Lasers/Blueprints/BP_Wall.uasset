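; BP_Wall is a wall built to shuttle its static mesh back and forth between two points, Loc1 and Loc2.
; WallMove waits briefly, then starts a looping timer that plays or reverses a timeline according to Arrived, which a FlipFlop toggles on each finish.
; Play rate is Speed over distance, keeping speed independent of path length.
; The setup capturing mesh and Target locations and calling WallMove is disconnected, and BeginPlay is empty.
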(event Custom|Move
  (Components|Timeline|SetPlayRate (Variables|Default|Get时间轴) (/ (Variables|Default|GetSpeed) (Math|Vector|VectorLength (- (Variables|Default|GetLoc2) (Variables|Default|GetLoc1)))))
  (if (Variables|Default|GetArrived?)
    (bind _新建轨道_0 (Timeline|时间轴 Reverse)
      (:Update
        (Transformation|SetWorldLocation (Variables|Default|GetStaticMesh) (+ (* (- (Variables|Default|GetLoc2) (Variables|Default|GetLoc1)) _新建轨道_0) (Variables|Default|GetLoc1)) false false))
      (:Finished
        (Utilities|FlowControl|FlipFlop
          (:A
            (Variables|Default|SetArrived? true))
          (:B
            (Variables|Default|SetArrived? false)))))
    (else
      (Timeline|时间轴 Play))))

(event Custom|WallMove
  (Utilities|FlowControl|Delay 1.0)
  (Utilities|Time|SetTimerbyEvent (delegate Custom|Move) 0.025 true))

(event EventBeginPlay)

(event Collision|EventActorBeginOverlap
  (params (OtherActor :type Actor%20Object%20Reference)))

(event EventTick
  (params (DeltaSeconds :type Float%20%28single-precision%29)))

(fn ConstructionScript)