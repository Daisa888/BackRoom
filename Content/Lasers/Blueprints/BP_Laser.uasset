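; BP_Laser is a colored laser beam actor that traces forward each tick and stretches its mesh to the blocking hit or full range.
; Hit actors with an AC_Handler component receive start, update and stop messages by comparing the current and previous frames' handler sets.
; A recursive walk through PreviousLasers skips handlers already upstream, preventing loops in chained beams.
; Color changes notify hit handlers, and LaserStop messages them before destroying the actor.
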(event EventBeginPlay
  (bind _returnvalue (Rendering|Material|CreateDynamicMaterialInstance "/Game/Lasers/Materials/MI_Laser.MI_Laser" "None" "None" :!class /Script/Engine.KismetMaterialLibrary))
  (Variables|Default|SetMI_Laser _returnvalue)
  (Rendering|Material|SetMaterial (Variables|Default|GetLaser) 0 (Variables|Default|GetMI_Laser))
  (CallFunction|SetLaserColor (Variables|Exposed|GetColorOverride)))

(event Collision|EventActorBeginOverlap
  (params (OtherActor :type Actor%20Object%20Reference)))

(event EventTick
  (params (DeltaSeconds :type Float%20%28single-precision%29))
  (bind _returnvalue (Transformation|GetActorLocation))
  (bind (_outhits _returnvalue_2) (Collision|MultiLineTraceByChannel _returnvalue (+ _returnvalue (* (Transformation|GetActorForwardVector) (Variables|Default|GetRange))) "TraceTypeQuery3" false (Variables|Default|GetActorsToIgnore) "ForOneFrame"))
  (if _returnvalue_2
    (for _array_element _outhits
      (Utilities|FlowControl|Sequence
        (:then_0
          (if (.bBlockingHit (Collision|BreakHitResult _array_element))
            (CallFunction|UpdateLength (.Distance (Collision|BreakHitResult _array_element)))))
        (:then_1
          (CallFunction|HandleHitActors _array_element))))
    (else
      (CallFunction|UpdateLength (Variables|Default|GetRange))))
  (bind _result (Utilities|Set|Difference (Variables|Default|GetPreviousHitHandler) (Variables|Default|GetCurrentHitHandler)))
  (bind _result_2 (Utilities|Set|ToArray _result))
  (for _array_element_2 _result_2
    (Class|INTLasers|LaserStop(Message) _array_element_2 self)
    (Utilities|Map|Remove (Variables|Default|GetHittingHandlers) _array_element_2))
  (Variables|Default|SetPreviousHitHandler (Variables|Default|GetCurrentHitHandler))
  (Utilities|Set|Clear (Variables|Default|GetCurrentHitHandler)))

(event EventLaserStop
  (params (Input :type BP%20Laser%20Object%20Reference))
  (Utilities|FlowControl|Sequence
    (:then_0
      (bind _result (Utilities|Set|ToArray (Variables|Default|GetPreviousHitHandler)))
      (for _array_element _result
        (Class|INTLasers|LaserStop(Message) _array_element self)))
    (:then_1
      (Actor|DestroyActor))))

(fn ConstructionScript)

(fn SetLaserColor
  (params (Value :type Linear%20Color%20Structure))
  (Variables|Exposed|SetColorOverride Value)
  (Rendering|Material|SetVectorParameterValue (Variables|Default|GetMI_Laser) "Color" Value :!class /Script/Engine.MaterialInstanceDynamic)
  (bind _result (Utilities|Set|ToArray (Variables|Default|GetPreviousHitHandler)))
  (for _array_element _result
    (Default|IntermediateChange _array_element self)))

(fn UpdateLength
  (params (InputPin :type Float%20%28single-precision%29))
  (if (not (Math|Float|NearlyEqual(Float) InputPin (Variables|Default|GetPreviousLength) 2.0))
    (bind _output_get (Variables|Default|SetPreviousLength InputPin))
    (Transformation|SetWorldScale3D (Variables|Default|GetLaser) (Math|Vector|MakeVector 0.1 0.1 (* _output_get 0.01)))))

(fn HandleHitActors
  (params (InputPin :type Hit%20Result%20Structure))
  (bind _hitactor (Collision|BreakHitResult InputPin))
  (bind _returnvalue (Actor|GetComponentbyClass _hitactor "/Game/Lasers/Blueprints/Component/AC_Handler.AC_Handler_C"))
  (Utilities|IsValid _returnvalue
    (:Is%20Valid
      (LocalVariables|SetL_Handler _returnvalue)
      (if (CallFunction|IsNotonPath (LocalVariables|GetL_Handler))
        (Utilities|Map|Add (Variables|Default|GetHittingHandlers) (LocalVariables|GetL_Handler) InputPin)
        (if (Utilities|Set|Contains (Variables|Default|GetPreviousHitHandler) (LocalVariables|GetL_Handler))
          (Default|LaserUpdate (LocalVariables|GetL_Handler) self InputPin)
          (else
            (Class|INTLasers|LaserStart(Message) (LocalVariables|GetL_Handler) self InputPin)))
        (Utilities|Set|Add (Variables|Default|GetCurrentHitHandler) (LocalVariables|GetL_Handler))))))

(fn IsNotonPath
  (params (InputHandler :type AC%20Handler%20Object%20Reference))
  (if (Utilities|Array|IsNotEmpty (Variables|Default|GetPreviousLasers))
    (for _array_element (Variables|Default|GetPreviousLasers)
      (bind _output_get (LocalVariables|SetL_CurrentLaser _array_element))
      (Utilities|IsValid _output_get
        (:Is%20Valid
          (if (== (Variables|BP_Laser_C|GetOwningHandler _output_get) InputHandler)
            (return false)
            (elif (not (CallFunction|IsNotonPath (LocalVariables|GetL_CurrentLaser) InputHandler))
              (return false))))
        (:Is%20Not%20Valid
          (return false))))
    (return true)
    (else
      (return true))))

(fn GetHitbyHandler
  (params (Key :type AC%20Handler%20Object%20Reference%20%28by%20ref%29))
  (bind _hittinghandlers (Variables|Default|GetHittingHandlers))
  (bind (_value _returnvalue) (Utilities|Map|Find _hittinghandlers Key))
  (return _value _returnvalue))