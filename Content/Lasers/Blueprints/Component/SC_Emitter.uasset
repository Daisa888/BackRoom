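; SC_Emitter is a scene component that emits a BP_Laser from its transform, driven by the owning actor's AC_Handler.
; Start, stop and intermediate-change events spawn or stop the attached laser according to handler activation or color-matching rules, with inversion flipping start and stop.
; Laser color comes from an override or the handler's visible color and updates the live beam.
; Force events allow direct activation, optionally conditional, and deactivation.
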(event EventBeginPlay
  (bind _returnvalue (Components|GetOwner))
  (bind _returnvalue_2 (Actor|GetComponentbyClass _returnvalue "/Game/Lasers/Blueprints/Component/AC_Handler.AC_Handler_C"))
  (Utilities|IsValid _returnvalue_2
    (:Is%20Valid
      (Variables|Default|SetOwningHandler _returnvalue_2))))

(event EventIntermediateChange
  (params (Modified :type BP%20Laser%20Object%20Reference))
  (if (not (Utilities|IsSystemInverted))
    (CallFunction|SetLaserColor)
    (if (CallFunction|CanSpawnLaser)
      (Variables|Default|GetAttachedLaser
        (:then)
        (:else
          (CallFunction|ActivateLaser)))
      (else
        (CallFunction|DeactivateLaser)))))

(event EventLaserStart
  (params (Input :type BP%20Laser%20Object%20Reference) (HitInfo :type Hit%20Result%20Structure))
  (if (Utilities|IsSystemInverted)
    (CallFunction|DeactivateLaser)
    (else
      (CallFunction|SetLaserColor)
      (if (CallFunction|CanSpawnLaser)
        (Variables|Default|GetAttachedLaser
          (:then)
          (:else
            (CallFunction|ActivateLaser)))))))

(event EventLaserStop
  (params (Input :type BP%20Laser%20Object%20Reference))
  (if (Utilities|IsSystemInverted)
    (CallFunction|ActivateLaser)
    (elif (not (CallFunction|CanSpawnLaser))
      (CallFunction|DeactivateLaser))))

(event EventForceActivation
  (params (ApplyCondtions :type Boolean))
  (if ApplyCondtions
    (CallFunction|SetLaserColor)
    (if (CallFunction|CanSpawnLaser)
      (Variables|Default|GetAttachedLaser :!label _label
        (:then)
        (:else
          (CallFunction|ActivateLaser))))
    (else
      (CallFunction|SetLaserColor)
      (goto _label))))

(event EventForceDeactivation
  (params (ApplyCondtions :type Boolean))
  (CallFunction|DeactivateLaser))

(fn DeactivateLaser
  (bind _attachedlaser (Variables|Default|GetAttachedLaser)
    (:then
      (Default|LaserStop _attachedlaser))
    (:else)))

(fn ActivateLaser
  (bind _returnvalue (Game|SpawnActorfromClass "/Game/Lasers/Blueprints/BP_Laser.BP_Laser_C" (Transformation|GetWorldTransform) "Undefined" "MultiplyWithRoot" 0 (Variables|Default|GetCurrentColor) (Variables|Default|GetMaxRange) (Utilities|GetFilteredLaser) (Variables|Default|GetOwningHandler) (Utilities|Array|MakeArray (Components|GetOwner)) 0))
  (bind _output_get (Variables|Default|SetAttachedLaser _returnvalue))
  (Transformation|AttachComponentToComponent _output_get self "None" "KeepWorld" "KeepWorld" "KeepWorld" false))

(fn SetLaserColor
  (Utilities|FlowControl|Sequence
    (:then_0
      (if (Variables|Default|GetUseOverride)
        (LocalVariables|SetL_TempColor (Variables|Default|GetOverrideColor))
        (elif (Utilities|Array|IsEmpty (Variables|/Game/Lasers/Blueprints/Component/AC_Handler.AC_Handler_C|GetFliteredLasers (Variables|Default|GetOwningHandler)))
          (LocalVariables|SetL_TempColor (Variables|Default|GetCurrentColor))
          (else
            (LocalVariables|SetL_TempColor (Default|GetVisableColor (Variables|Default|GetOwningHandler)))))))
    (:then_1
      (if (!= (Variables|Default|GetCurrentColor) (LocalVariables|GetL_TempColor))
        (Variables|Default|SetCurrentColor (LocalVariables|GetL_TempColor))
        (bind _attachedlaser (Variables|Default|GetAttachedLaser)
          (:then
            (Default|SetLaserColor _attachedlaser (Variables|Default|GetCurrentColor)))
          (:else))))))

(fn CanSpawnLaser
  (bind _owninghandler (Variables|Default|GetOwningHandler))
  (if (Variables|/Game/Lasers/Blueprints/Component/AC_Handler.AC_Handler_C|GetIsAdjustingColor (Variables|Default|GetOwningHandler))
    (if (Variables|/Game/Lasers/Blueprints/Component/AC_Handler.AC_Handler_C|GetCanMergeColor (Variables|Default|GetOwningHandler))
      (return (Default|DoesContainColor _owninghandler (Default|GetMergeColor _owninghandler) (Variables|Default|GetOverrideColor)))
      (else
        (for _array_element (Utilities|GetFilteredLaser)
          (if (Default|DoesContainColor (Variables|Default|GetOwningHandler) (Variables|/Game/Lasers/Blueprints/BP_Laser.BP_Laser_C|GetColorOverride _array_element) (Variables|Default|GetOverrideColor))
            (return true)))
        (return false)))
    (else
      (return (Default|CanActivate (Variables|Default|GetOwningHandler))))))

(fn DestroySelf
  (Components|DestroyComponent))