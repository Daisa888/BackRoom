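; AC_Bounce is a laser component that bounces incoming beams off its owner by spawning a new SC_Emitter for each one.
; A map pairs each input laser with its bounced emitter, which is repositioned from mirrored hit data on update and destroyed on stop.
; Bounced emitters can inherit the incoming color.
; Forced activation or deactivation replays start or stop over the sibling AC_Handler's filtered lasers.
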(event EventBeginPlay
  (bind _returnvalue (Components|GetOwner))
  (bind _returnvalue_2 (Actor|GetComponentbyClass _returnvalue "/Game/Lasers/Blueprints/Component/AC_Handler.AC_Handler_C"))
  (Utilities|IsValid _returnvalue_2
    (:Is%20Valid
      (Variables|Default|SetOwningHandler _returnvalue_2))))

(event EventTick
  (params (DeltaSeconds :type Float%20%28single-precision%29)))

(event EventLaserStart
  (params (Input :type BP%20Laser%20Object%20Reference) (HitInfo :type Hit%20Result%20Structure))
  (Utilities|IsValid Input
    (:Is%20Valid
      (if (not (Utilities|Map|Contains (Variables|Default|GetEmitterBounceMap) Input))
        (CallFunction|SpawnLaser Input HitInfo)))))

(event EventLaserStop
  (params (Input :type BP%20Laser%20Object%20Reference))
  (CallFunction|RemoveLaser Input))

(event EventLaserUpdate
  (params (Input :type BP%20Laser%20Object%20Reference) (HitInfo :type Hit%20Result%20Structure))
  (bind (_loction _rotion) (Utilities|MirrorLocationandRotation HitInfo))
  (bind _emitterbouncemap (Variables|Default|GetEmitterBounceMap))
  (bind (_value _returnvalue) (Utilities|Map|Find _emitterbouncemap Input))
  (if _returnvalue
    (Transformation|SetWorldLocationAndRotation _value _loction _rotion false false)))

(event EventIntermediateChange
  (params (Modified :type BP%20Laser%20Object%20Reference))
  (bind _values (Utilities|Map|Values (Variables|Default|GetEmitterBounceMap)))
  (for _array_element _values
    (Default|SetLaserColor _array_element)))

(event EventForceActivation
  (params (ApplyCondtions :type Boolean))
  (for _array_element (Variables|/Game/Lasers/Blueprints/Component/AC_Handler.AC_Handler_C|GetFliteredLasers (Variables|Default|GetOwningHandler))
    (if (.ReturnValue (Default|GetHitbyHandler _array_element (Variables|Default|GetOwningHandler)))
      (CallFunction|LaserStart _array_element (.Value (Default|GetHitbyHandler _array_element (Variables|Default|GetOwningHandler)))))))

(event EventForceDeactivation
  (params (ApplyCondtions :type Boolean))
  (for _array_element (Variables|/Game/Lasers/Blueprints/Component/AC_Handler.AC_Handler_C|GetFliteredLasers (Variables|Default|GetOwningHandler))
    (CallFunction|LaserStop _array_element)))

(fn SpawnLaser
  (params (LaserIn :type BP%20Laser%20Object%20Reference) (HitInfo :type Hit%20Result%20Structure))
  (bind _returnvalue (Components|GetOwner))
  (bind _returnvalue_2 (Transformation|GetActorTransform _returnvalue))
  (bind (_loction _rotion) (Utilities|MirrorLocationandRotation HitInfo))
  (bind _returnvalue_3 (Game|AddComponentbyClass (Components|GetOwner) "/Game/Lasers/Blueprints/Component/SC_Emitter.SC_Emitter_C" false (Math|Transform|MakeTransform (Math|Transform|InverseTransformLocation _returnvalue_2 _loction) (Math|Transform|InverseTransformRotation _returnvalue_2 _rotion) "1.000000,1.000000,1.000000")))
  (Utilities|Map|Add (Variables|Default|GetEmitterBounceMap) LaserIn _returnvalue_3)
  (if (Variables|Default|GetUseBounceColor)
    (Variables|/Game/Lasers/Blueprints/Component/SC_Emitter.SC_Emitter_C|SetOverrideColor _returnvalue_3 (Variables|/Game/Lasers/Blueprints/BP_Laser.BP_Laser_C|GetColorOverride LaserIn))
    (Variables|/Game/Lasers/Blueprints/Component/SC_Emitter.SC_Emitter_C|SetUseOverride _returnvalue_3 true))
  (Default|SetLaserColor _returnvalue_3)
  (Default|ActivateLaser _returnvalue_3))

(fn RemoveLaser
  (params (InputPin :type BP%20Laser%20Object%20Reference))
  (bind _emitterbouncemap (Variables|Default|GetEmitterBounceMap))
  (bind (_value _returnvalue) (Utilities|Map|Find _emitterbouncemap InputPin))
  (if _returnvalue
    (bind _output_get (LocalVariables|SetL_RemoveItem _value))
    (Default|ForceDeactivation _output_get false)
    (Utilities|Map|Remove (Variables|Default|GetEmitterBounceMap) InputPin)
    (Default|DestroySelf (LocalVariables|GetL_RemoveItem))))