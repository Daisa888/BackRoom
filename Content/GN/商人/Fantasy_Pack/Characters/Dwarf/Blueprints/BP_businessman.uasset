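; BP_businessman is a dwarf merchant NPC that reacts to a nearby player through its animation Blueprint.
; BeginPlay caches the ABP_Businessman instance from the SKDwarf mesh.
; A sphere overlap with a MyCharacterBase stores it as Player and switches to the approach state, while any overlap end switches to leave and clears Player.
; The Purchase event switches to the purchase state only while Player is valid, with no transaction logic here.
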(event OnComponentBeginOverlap(Sphere)
  (params (OverlappedComponent :type Primitive%20Component%20Object%20Reference) (OtherActor :type Actor%20Object%20Reference) (OtherComp :type Primitive%20Component%20Object%20Reference) (OtherBodyIndex :type Integer) (bFromSweep :type Boolean) (SweepResult :type Hit%20Result%20Structure%20%28by%20ref%29))
  (bind _asmy_character_base (Utilities|Casting|CastToMyCharacterBase OtherActor))
  (Variables|Default|Setplayer _asmy_character_base)
  (Default|ChangeAction (Variables|Default|Getbusinessman%20Animation) true false false))

(event OnComponentEndOverlap(Sphere)
  (params (OverlappedComponent :type Primitive%20Component%20Object%20Reference) (OtherActor :type Actor%20Object%20Reference) (OtherComp :type Primitive%20Component%20Object%20Reference) (OtherBodyIndex :type Integer))
  (Default|ChangeAction (Variables|Default|Getbusinessman%20Animation) false false true)
  (Variables|Default|Setplayer 0))

(event EventBeginPlay
  (bind _asabp_businessman (Utilities|Casting|CastToABP_Businessman (Components|SkeletalMesh|GetAnimInstance (Variables|Default|GetSK_Dwarf))))
  (Variables|Default|Setbusinessman%20Animation _asabp_businessman))

(event Collision|EventActorBeginOverlap
  (params (OtherActor :type Actor%20Object%20Reference)))

(event EventTick
  (params (DeltaSeconds :type Float%20%28single-precision%29)))

(event EventPurchase
  (Utilities|IsValid (Variables|Default|Getplayer)
    (:Is%20Valid
      (Default|ChangeAction (Variables|Default|Getbusinessman%20Animation) true true false))))

(fn ConstructionScript)