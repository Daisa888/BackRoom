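; BP_Cabinet is a drawer-sequence puzzle: clicked meshes must match a set order, and a wrong pick resets progress.
; A cabinet without a TargetCabinet shuffles CubeArray and locks itself; one with a target copies that order by matching component names.
; Valid clicks slide the mesh out along its right vector and back via two timelines, with input briefly blocked.
; Completion only prints a placeholder message and disables pulling.
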(event Custom|PullOut
  (params (目标 :type Scene%20Component%20Object%20Reference))
  (bind _returnvalue (Transformation|GetWorldLocation 目标))
  (if (CallFunction|CanPullOut? 目标)
    (Variables|Default|SetLoc1 _returnvalue)
    (Variables|Default|SetLoc2 (+ _returnvalue (* (Math|Vector|GetRightVector 目标) "100.000000,100.000000,100.000000")))
    (Utilities|Time|SetTimerbyEvent (delegate Custom|Move) 0.025)))

(event Custom|Move
  (Components|Timeline|SetPlayRate (Variables|Default|Get时间轴) (/ (Variables|Default|GetSpeed) (Math|Vector|VectorLength (- (Variables|Default|GetLoc2) (Variables|Default|GetLoc1)))))
  (bind _新建轨道_0 (Timeline|时间轴 PlayFromStart)
    (:Update
      (Transformation|SetWorldLocation (stale Custom|PullOut 目标) (+ (* (- (Variables|Default|GetLoc2) (Variables|Default|GetLoc1)) _新建轨道_0) (Variables|Default|GetLoc1)) false false))
    (:Finished
      (Utilities|FlowControl|Delay 0.2)
      (bind _新建轨道_0_2 (Timeline|时间轴_0 PlayFromStart)
        (:Update
          (Transformation|SetWorldLocation (stale Custom|PullOut 目标) (+ (* (- (Variables|Default|GetLoc1) (Variables|Default|GetLoc2)) _新建轨道_0_2) (Variables|Default|GetLoc2)) false false))))))

(event EventBeginPlay
  (bind _targetcabinet (Variables|默认|GetTargetCabinet))
  (Variables|Default|SetCubeArray (Utilities|Array|MakeArray (Variables|Default|Get1) (Variables|Default|Get2) (Variables|Default|Get3)))
  (Utilities|IsValid _targetcabinet
    (:Is%20Valid
      (for _array_element (Variables|BP_Cabinet_C|GetCubeArray _targetcabinet)
        (for _array_element_2 (Variables|Default|GetCubeArray)
          (if (Utilities|Enum|Equal(Enum) (Utilities|GetObjectName _array_element) (Utilities|GetObjectName _array_element_2))
            (Utilities|Array|Add (Variables|Default|GetTempArray) _array_element_2))))
      (Variables|Default|SetCubeArray (Variables|Default|GetTempArray)))
    (:Is%20Not%20Valid
      (Utilities|Array|Shuffle (Variables|Default|GetCubeArray))
      (Variables|Default|SetLockTargetCabinet? true))))

(event Collision|EventActorBeginOverlap
  (params (OtherActor :type Actor%20Object%20Reference)))

(event EventTick
  (params (DeltaSeconds :type Float%20%28single-precision%29)))

(event EventClicked
  (params (C :type Scene%20Component%20Object%20Reference) (O :type Actor%20Object%20Reference))
  (bind _cubearray (Variables|Default|GetCubeArray))
  (if (== (Utilities|Array|Length (Variables|Default|GetCubeArray)) (Variables|Default|GetCorrectNumber))
    (Development|PrintString "ok")
    (elif (and (CallFunction|CanPullOut? C) (Variables|Default|GetCanPull?))
      (if (not (Variables|Default|GetLockTargetCabinet?))
        (Variables|Default|SetTempSC C)
        (Variables|Default|SetCanPull? false)
        (CallFunction|PullOut (Variables|Default|GetTempSC))
        (Utilities|FlowControl|Delay 2.0)
        (Variables|Default|SetCanPull? true)
        (if (Utilities|Enum|Equal(Enum) (Utilities|GetObjectName (Utilities|Array|Get(acopy) _cubearray (Variables|Default|GetCorrectNumber))) (Utilities|GetObjectName (Variables|Default|GetTempSC)))
          (bind _output_get (Variables|Default|SetCorrectNumber (+ (Variables|Default|GetCorrectNumber) 1)))
          (Development|PrintString (Utilities|String|ToString(Integer) _output_get))
          (if (== (+ (Utilities|Array|Length _cubearray) 1) (+ (Variables|Default|GetCorrectNumber) 1))
            (Development|PrintString "完成 执行后续逻辑")
            (Variables|Default|SetCanPull? false))
          (else
            (bind _output_get_2 (Variables|Default|SetCorrectNumber 0))
            (Development|PrintString (Utilities|String|ToString(Integer) _output_get_2))))))))

(fn ConstructionScript)

(fn Open)

(fn CanPullOut?
  (params (SC :type Scene%20Component%20Object%20Reference))
  (bind _as静态网格体组件 (Utilities|Casting|CastToStaticMeshComponent SC)
    (:then
      (if (== (Utilities|Array|FindItem (Variables|Default|GetCubeArray) _as静态网格体组件) -1)
        (return false)
        (else
          (return true))))
    (:CastFailed
      (return false))))